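; Base enemy AI controller that runs the BT_EnemyBase behavior tree on possession.
; On possess it initializes target, stun and combat-ability flags in BB_Enemy_Base and starts a looping timer that writes the TargetActor key with no value supplied.
; AI Perception updates controller variables for target, line of sight and last known location, but clears TargetActor on detection and never copies these variables to the blackboard.
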(event OnTargetPerceptionUpdated(AIPerception)
  (params (Actor :type Actor%20Object%20Reference) (Stimulus :type AI%20Stimulus%20Structure))
  (if (.bSuccessfullySensed (Utilities|Struct|BreakAIStimulus Stimulus))
    (bind _asbp_third_person_character (Utilities|Casting|CastTo Actor)
      (:then
        (Variables|Default|SetTargetActor 0)
        (Variables|Default|SetbHasTarget true)
        (Variables|Default|SetbHasLOS true)
        (Variables|Default|SetLastKnownLocation (Transformation|GetActorLocation _asbp_third_person_character)))
      (:CastFailed
        (Utilities|String|LogString "没检测到玩家")))
    (else
      (Variables|Default|SetbHasLOS false)
      (Variables|Default|SetbHasTarget (Utilities|IsValid (Variables|Default|GetTargetActor))))))

(event Custom|UpdateBlackboardDistance
  (Class|AIController|UseBlackboard "/Game/Enemy/AI/BB_Enemy_Base.BB_Enemy_Base")
  (AI|Components|Blackboard|SetValueasObject (Utilities|Name|MakeLiteralName "TargetActor") 0))

(event EventBeginPlay
  (Utilities|String|LogString "启动通用敌人AI"))

(event EventPossess
  (params (PossessedPawn :type Pawn%20Object%20Reference))
  (Utilities|FlowControl|Sequence
    (:then_0
      (AI|RunBehaviorTree "/Game/Enemy/AI/BT_EnemyBase.BT_EnemyBase")
      (bind _blackboardcomponent (Class|AIController|UseBlackboard "/Game/Enemy/AI/BB_Enemy_Base.BB_Enemy_Base"))
      (AI|Components|Blackboard|SetValueasBool _blackboardcomponent (Utilities|Name|MakeLiteralName "bHasTarget") false)
      (AI|Components|Blackboard|SetValueasBool _blackboardcomponent (Utilities|Name|MakeLiteralName "bHasLOS") false)
      (AI|Components|Blackboard|SetValueasBool _blackboardcomponent (Utilities|Name|MakeLiteralName "bIsStunnrd") false)
      (AI|Components|Blackboard|SetValueasBool _blackboardcomponent (Utilities|Name|MakeLiteralName "bCanMelee") true)
      (AI|Components|Blackboard|SetValueasBool _blackboardcomponent (Utilities|Name|MakeLiteralName "bCanRange") true)
      (AI|Components|Blackboard|SetValueasBool _blackboardcomponent (Utilities|Name|MakeLiteralName "bCanCharge") true)
      (AI|Components|Blackboard|SetValueasBool _blackboardcomponent (Utilities|Name|MakeLiteralName "bCanRetreat") true))
    (:then_1
      (Utilities|Time|SetTimerbyEvent (delegate Custom|UpdateBlackboardDistance) 0.2 true))))

(fn ConstructionScript)